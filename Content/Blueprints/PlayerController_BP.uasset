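; Player controller that handles keyboard movement of the player character and a mouse-click debug readout.
; MoveForward and MoveRight axis inputs feed AddMovementInput along the camera manager's forward and right vectors, making movement camera-relative.
; A left mouse press runs a complex Visibility trace under the cursor and prints the display name of the hit actor in green.
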(event Input|AxisEvents|InputAxisMoveForward
  (params (AxisValue :type Float%20%28single-precision%29))
  ;[1 1 1] WASD Controlls
  (Pawn|Input|AddMovementInput (Game|GetPlayerCharacter 0) (Transformation|GetActorForwardVector (Game|GetPlayerCameraManager 0)) AxisValue false))

(event Input|AxisEvents|InputAxisMoveRight
  (params (AxisValue :type Float%20%28single-precision%29))
  ;[1 1 1] WASD Controlls
  (Pawn|Input|AddMovementInput (Game|GetPlayerCharacter 0) (Transformation|GetActorRightVector (Game|GetPlayerCameraManager 0)) AxisValue false))

(event Input|MouseEvents|LeftMouseButton
  (params (Key :type Key%20Structure :default "AnyKey"))
  ;[1 1 1] Print name of clicked object
  (:Pressed
    (Development|PrintString (Utilities|GetDisplayName (.HitActor (Collision|BreakHitResult (.HitResult (Game|Player|GetHitResultUnderCursorbyChannel "TraceTypeQuery1" true))))) true true "(R=0.000000,G=1.000000,B=0.082511,A=1.000000)")))

(fn ConstructionScript)